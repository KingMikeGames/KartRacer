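; FPSCounter is a Blueprint that displays the current frame rate on FpsText, in the QualityMenu example room.
; Each Tick blends DeltaSeconds into a stored value with a low-alpha Lerp, giving a smoothed frame time.
; The inverse of that value, nudged by a small offset to stop flicker on whole numbers, is written to the text with an "FPS:" prefix.
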(event EventBeginPlay)

(event EventActorBeginOverlap
  (params (OtherActor :type Actor%20Object%20Reference)))

(event EventTick
  (params (DeltaSeconds :type Float%20%28single-precision%29))
  (Variables|Default|SetLerptarget (Math|Float|Lerp (Variables|Default|GetLerptarget) DeltaSeconds 0.02))
  (Rendering|Components|TextRender|SetText (Variables|Default|GetFpsText) (Utilities|Text|ToText(String) (Utilities|String|Append "FPS:" (Utilities|String|ToString(Text) (Utilities|Text|ToText(Float) (+ (/ 1.0 (Variables|Default|GetLerptarget)) 0.03) "HalfToEven" true 1 324 2 2))))))

(fn ConstructionScript)