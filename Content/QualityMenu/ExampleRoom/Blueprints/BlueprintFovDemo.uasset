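; Demo actor that animates a scene capture camera's field of view and visualizes the changing angle.
; Each Tick, a sine-based math expression of game time sets the capture component's FOV.
; Two scene components yaw by plus and minus half that angle to follow the horizontal view edges, while a text render displays the current value.
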(event EventBeginPlay)

(event EventTick
  (params (DeltaSeconds :type Float%20%28single-precision%29))
  (bind _returnvalue (Utilities|Time|GetGameTimeinSeconds))
  (bind _returnvalue_2 (|(50+(((sin(x))+1)*30)) _returnvalue))
  (Variables|/Script/Engine.SceneCaptureComponent2D|SetFOVAngle (Variables|DecalActor|GetCaptureComponent2D) _returnvalue_2)
  (Transformation|SetRelativeRotation (Variables|Default|GetScene) (Math|Rotator|MakeRotator 0.0 0.0 (/ _returnvalue_2 2.0)) false false)
  (Transformation|SetRelativeRotation (Variables|Default|GetScene1) (Math|Rotator|MakeRotator 0.0 0.0 (/ _returnvalue_2 -2.0)) false false)
  (Rendering|Components|TextRender|SetText (Variables|Default|GetTextRender) (Utilities|Text|ToText(String) (Utilities|String|Append "FOV: " (Utilities|String|ToString(Text) (Utilities|Text|ToText(Float) _returnvalue_2 "HalfToEven" true 1 324 0 0))))))

(fn ConstructionScript)