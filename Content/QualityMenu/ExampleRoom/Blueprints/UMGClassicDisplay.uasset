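; Example-room display actor that shows the classic settings menu in a widget component, opened on a chosen tab.
; The WidgetDisplay option selects the Audio, Video, Mouse or Game tab, and the construction script applies it through SwitchTab.
; BeginPlay repeats the switch after a short delay to avoid a visual race, but passes a fixed widget index of 1 instead of WidgetDisplay.
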(event EventBeginPlay
  (Utilities|FlowControl|Delay 0.05) ; Fix Visual Race condition in this example
  (bind _asclassic_settings_menu_main (Utilities|Casting|CastToClassicSettingsMenuMain (UserInterface|GetUserWidgetObject (Variables|Default|GetWidget))))
  (Default|SwitchTab _asclassic_settings_menu_main (Utilities|Select :Index (Variables|Default|GetWidgetDisplay) :Option%200 (Variables|/Game/QualityMenu/HUD_UMG_Classic/ClassicSettingsMenuMain.ClassicSettingsMenuMain_C|GetTab%20Audio%20Settings _asclassic_settings_menu_main) :Option%201 (Variables|/Game/QualityMenu/HUD_UMG_Classic/ClassicSettingsMenuMain.ClassicSettingsMenuMain_C|GetTab%20Video%20Settings _asclassic_settings_menu_main) :Option%202 (Variables|/Game/QualityMenu/HUD_UMG_Classic/ClassicSettingsMenuMain.ClassicSettingsMenuMain_C|GetTab%20Mouse%20Settings _asclassic_settings_menu_main) :Option%203 (Variables|/Game/QualityMenu/HUD_UMG_Classic/ClassicSettingsMenuMain.ClassicSettingsMenuMain_C|GetTab%20Game%20Settings _asclassic_settings_menu_main)) 1))

(event Collision|EventActorBeginOverlap
  (params (OtherActor :type Actor%20Object%20Reference)))

(event EventTick
  (params (DeltaSeconds :type Float%20%28single-precision%29)))

(fn ConstructionScript
  (bind _widgetdisplay (Variables|Default|GetWidgetDisplay))
  (bind _asclassic_settings_menu_main (Utilities|Casting|CastToClassicSettingsMenuMain (UserInterface|GetUserWidgetObject (Variables|Default|GetWidget))))
  (Default|SwitchTab _asclassic_settings_menu_main (Utilities|Select :Index _widgetdisplay :Option%200 (Variables|/Game/QualityMenu/HUD_UMG_Classic/ClassicSettingsMenuMain.ClassicSettingsMenuMain_C|GetTab%20Audio%20Settings _asclassic_settings_menu_main) :Option%201 (Variables|/Game/QualityMenu/HUD_UMG_Classic/ClassicSettingsMenuMain.ClassicSettingsMenuMain_C|GetTab%20Video%20Settings _asclassic_settings_menu_main) :Option%202 (Variables|/Game/QualityMenu/HUD_UMG_Classic/ClassicSettingsMenuMain.ClassicSettingsMenuMain_C|GetTab%20Mouse%20Settings _asclassic_settings_menu_main) :Option%203 (Variables|/Game/QualityMenu/HUD_UMG_Classic/ClassicSettingsMenuMain.ClassicSettingsMenuMain_C|GetTab%20Game%20Settings _asclassic_settings_menu_main)) _widgetdisplay))