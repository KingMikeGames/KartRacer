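; Actor that acts as the Quality Menu's global post process controller, applying the saved gamma, bloom and gain settings to its PostProcess component.
; On BeginPlay it reads game settings and registers itself with the GameInstance, applying values on success or printing an error and deactivating if refused.
; Its interface functions update each effect individually, or deactivate the component and change its text label when another controller replaces it.
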(event EventBeginPlay
  (bind _game_settings (Utilities|GetGameSettings (Game|GetGameInstance))
    (:Out
      (Variables|Default|SetGameSettings _game_settings)
      (bind _replaced (Utilities|SetGlobalPostProcess (Game|GetGameInstance) self)
        (:Out
          (if _replaced
            (CallFunction|UpdateGlobalPostEffects)
            (else
              (Development|PrintString "Error: GobalPostProcessSetting. Global Post Process setting contoller exists in Game settings and did not want to be replaced")
              (Components|Activation|Deactivate (Variables|Default|GetPostProcess)))))))))

(fn ConstructionScript)

(fn UpdateGlobalPostEffects
  (bind _gamesettings (Variables|Default|GetGameSettings))
  (CallFunction|UpdateGamma (Variables|/Game/QualityMenu/Blueprints/GameSettings.GameSettings_C|GetGamma%20Strength _gamesettings))
  (CallFunction|UpdateBloom (Variables|/Game/QualityMenu/Blueprints/GameSettings.GameSettings_C|GetBloom%20Strength _gamesettings))
  (CallFunction|UpdateGain (Variables|/Game/QualityMenu/Blueprints/GameSettings.GameSettings_C|GetGain%20Strength _gamesettings)))

(fn ReplaceGlobalPostProcess
  (params (New%20Global%20Post%20Process :type Global%20Post%20Process%20Interface%20Interface))
  (if (== (Utilities|ToObject(Interface) New%20Global%20Post%20Process) self) ; Do not replace post process if its the same
    _
    (else
      (Components|Activation|Deactivate (Variables|Default|GetPostProcess))
      (Rendering|Components|TextRender|SetText (Variables|Default|GetTextRender) (Utilities|Text|MakeLiteralText "Quality Menu 
Global Post Process 
Deactivated"))))
  (return true))

(fn UpdateBloom
  (params (Bloom%20Strength :type Float%20%28single-precision%29))
  (Utilities|Struct|SetmembersinPostProcessSettings (Variables|/Script/Engine.PostProcessComponent|GetSettings (Variables|Default|GetPostProcess)) Bloom%20Strength)
  (return false))

(fn UpdateGain
  (params (Gain%20Strength :type Float%20%28single-precision%29))
  (Utilities|Struct|SetmembersinPostProcessSettings (Variables|/Script/Engine.PostProcessComponent|GetSettings (Variables|Default|GetPostProcess)) (Math|Conversions|ToVector(Float) Gain%20Strength))
  (return false))

(fn UpdateGamma
  (params (Gamma%20Strength :type Float%20%28single-precision%29))
  (Utilities|Struct|SetmembersinPostProcessSettings (Variables|/Script/Engine.PostProcessComponent|GetSettings (Variables|Default|GetPostProcess)) (Math|Conversions|ToVector(Float) Gamma%20Strength))
  (return false))