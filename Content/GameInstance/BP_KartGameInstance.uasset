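; Game instance for a kart game that holds the game settings object and the persistent player info for the session.
; On Init it creates the settings object with itself as the settings interface, then loads or creates the PlayerInfo save.
; SaveGame writes player info back to its slot and also runs on Shutdown.
; Helper functions expose the settings instance and execute console commands.
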(event Custom|SaveGame
  (Variables|/Game/SaveGame/PlayerInfoSave.PlayerInfoSave_C|SetPlayerInfo (Variables|Default|GetSave) (Variables|Default|GetPlayerInfo))
  (SaveGame|SaveGametoSlot (Variables|Default|GetSave) "PlayerInfo"))

(event EventInit
  (bind _game_settings (Utilities|InitGameSettings "SettingsSaveFile" 0 self)
    (:Out
      (Variables|Default|SetGame%20Settings _game_settings)
      (bind _returnvalue (SaveGame|LoadGamefromSlot "PlayerInfo"))
      (Utilities|IsValid _returnvalue
        (:Is%20Valid
          (bind _asplayer_info_save (Utilities|Casting|CastToPlayerInfoSave _returnvalue))
          (bind _output_get (Variables|Default|SetSave _asplayer_info_save))
          (Variables|Default|SetPlayerInfo (Variables|/Game/SaveGame/PlayerInfoSave.PlayerInfoSave_C|GetPlayerInfo _output_get)))
        (:Is%20Not%20Valid
          (bind _returnvalue_2 (SaveGame|CreateSaveGameObject "/Game/SaveGame/PlayerInfoSave.PlayerInfoSave_C"))
          (bind _asplayer_info_save_2 (Utilities|Casting|CastToPlayerInfoSave _returnvalue_2))
          (Variables|Default|SetSave _asplayer_info_save_2))))))

(event EventShutdown
  (CallFunction|SaveGame))

(fn GetSettingsInstance
  (return (Variables|Default|GetGame%20Settings)))

(fn RunConsoleCommand
  (params (Console%20Command :type String))
  (Development|ExecuteConsoleCommand Console%20Command)
  (return false))