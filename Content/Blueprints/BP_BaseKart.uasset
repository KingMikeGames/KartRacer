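; BP_BaseKart is a work-in-progress hover kart that accelerates along its forward arrow from axis input.
; Each tick it derives and debug-draws a plane from three wheel positions, then integrates velocity by teleporting the mesh, easing to zero without throttle.
; When any WheelComponent reports grounded, it lifts the mesh once along the plane normal and disables gravity.
; Turn input and rotation updates are empty stubs.
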(event EventTick
  (params (DeltaSeconds :type Float%20%28single-precision%29))
  (CallFunction|CalculatePlane)
  (CallFunction|UpdateKartRotation)
  (CallFunction|UpdateVelocity)
  (bind _grounded (CallFunction|GroundCheck))
  (if _grounded
    (if (not (Variables|Default|GetHovering))
      (Transformation|AddWorldOffset (Variables|Default|GetKartMesh) (* (Variables|Default|GetPlaneNormal) 25.0) false true)
      (Variables|Default|SetHovering true)
      (Physics|SetEnableGravity (Variables|Default|GetKartMesh) false))))

(event EventBeginPlay
  (CallFunction|CalculatePlane))

(event Input|AxisEvents|InputAxisAccelerate
  (params (AxisValue :type Float%20%28single-precision%29))
  (CallFunction|Accelerate AxisValue))

(event Input|AxisEvents|InputAxisTurn
  (params (AxisValue :type Float%20%28single-precision%29)))

(fn ConstructionScript)

(fn CalculatePlane
  (bind _backrightwheel (Variables|Default|GetBackRightWheel))
  (bind _returnvalue (Transformation|GetWorldLocation _backrightwheel))
  (bind _output_get (Variables|Default|SetPlaneNormal (Math|Vector|Normalize (Math|Vector|CrossProduct (- _returnvalue (Transformation|GetWorldLocation (Variables|Default|GetBackLeftWheel))) (- _returnvalue (Transformation|GetWorldLocation (Variables|Default|GetFrontRightWheel)))))))
  (bind _output_get_2 (Variables|Default|SetPlane (Utilities|Struct|MakePlane (Math|Vector|DotProduct _output_get (Transformation|GetWorldLocation (Variables|Default|GetBackLeftWheel))) (.X (Math|Vector|BreakVector (Variables|Default|GetPlaneNormal))) (.Y (Math|Vector|BreakVector (Variables|Default|GetPlaneNormal))) (.Z (Math|Vector|BreakVector (Variables|Default|GetPlaneNormal))))))
  (Class|KismetSystemLibrary|DrawDebugPlane _output_get_2 (Transformation|GetWorldLocation (Variables|Default|GetPlaneLocation)) 5e+01 "(R=1.000000,G=0.000000,B=0.689363,A=1.000000)" (Utilities|Time|GetWorldDeltaSeconds)))

(fn Accelerate
  (params (Axis%20Value :type Float%20%28single-precision%29))
  (bind _returnvalue (< Axis%20Value 0.0))
  (Variables|Default|SetAccelerating (not (== Axis%20Value 0.0)))
  (Variables|Default|SetReversing _returnvalue)
  (if (or (and _returnvalue (> (Variables|Default|GetAcceleration) 0.0)) (and (> Axis%20Value 0.0) (< (Variables|Default|GetAcceleration) 0.0)))
    (Variables|Default|SetAcceleration (* (Variables|Default|GetAcceleration) -1.0))))

(fn UpdateVelocity
  (if (Variables|Default|GetAccelerating)
    (if (< (Math|Vector|VectorLength (Variables|Default|GetVelocity)) (Variables|Default|GetMaxSpeed))
      (bind _output_get (Variables|Default|SetVelocity (+ (Variables|Default|GetVelocity) (* (Math|Vector|GetForwardVector (Variables|Default|GetForwardArrow)) (Variables|Default|GetAcceleration)))))
      (Transformation|SetWorldLocation (Variables|Default|GetKartMesh) (+ (* _output_get (Utilities|Time|GetWorldDeltaSeconds)) (Transformation|GetWorldLocation (Variables|Default|GetKartMesh))) false true)
      (else
        (Transformation|SetWorldLocation (Variables|Default|GetKartMesh) (+ (* (Variables|Default|GetVelocity) (Utilities|Time|GetWorldDeltaSeconds)) (Transformation|GetWorldLocation (Variables|Default|GetKartMesh))) false true)))
    (else
      ;[1 1 1] If !Accelerating, lerp velocity toward 0
      (bind _output_get_2 (Variables|Default|SetVelocity (Math|Vector|Lerp(Vector) (Variables|Default|GetVelocity) "0, 0, 0" (Variables|Default|GetDecelerationRate))))
      (Transformation|SetWorldLocation (Variables|Default|GetKartMesh) (+ (* _output_get_2 (Utilities|Time|GetWorldDeltaSeconds)) (Transformation|GetWorldLocation (Variables|Default|GetKartMesh))) false true))))

(fn UpdateKartRotation)

(fn GroundCheck
  (bind _numberofwheelsgrounded (LocalVariables|GetNumberofWheelsGrounded))
  (for _array_element (Components|GetChildrenComponents (Variables|Default|GetWheels) false)
    (bind _aswheel_component (Utilities|Casting|CastToWheelComponent _array_element))
    (if (Variables|/Game/Blueprints/WheelComponent.WheelComponent_C|GetGrounded _aswheel_component)
      (Math|Integer|IncrementInt (LocalVariables|GetNumberofWheelsGrounded))))
  (Development|PrintString (Utilities|String|ToString(Integer) _numberofwheelsgrounded))
  (return (> _numberofwheelsgrounded 0)))