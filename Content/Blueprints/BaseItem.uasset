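; BaseItem is a base actor for kart items, with stub UseItem, Throw and Activate functions that supply the interface but no behavior.
; ApplyGravity averages the inverted up vectors of overlapping GravityVolume actors into a normalized direction, falling back to world down when none overlap.
; It then pushes ItemMesh along that direction as a mass-independent acceleration scaled by GravityStrength, though nothing in this Blueprint calls it.
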(event EventBeginPlay)

(event EventActorBeginOverlap
  (params (OtherActor :type Actor%20Object%20Reference)))

(event EventTick
  (params (DeltaSeconds :type Float%20%28single-precision%29)))

(fn ConstructionScript)

(fn UseItem
  (params (ControllerLeftStickX :type Float%20%28single-precision%29) (ControllerLeftStickY :type Float%20%28single-precision%29) (ParentRotation :type Rotator) (ParentVelocity :type Vector))
  (return false))

(fn Throw
  (params (ControllerLeftStickX :type Float%20%28single-precision%29) (ControllerLeftStickY :type Float%20%28single-precision%29) (ParentRotation :type Rotator) (ParentVelocity :type Vector)))

(fn Activate
  (params (KartReference :type BP%20Kart%203%20Object%20Reference))
  (return false))

(fn ApplyGravity
  (bind _overlappingactors (Collision|GetOverlappingActors "/Game/Blueprints/GravityVolume.GravityVolume_C" :!class /Script/Engine.Actor))
  (Utilities|FlowControl|Sequence
    (:then_0
      ;[1 1 1] Determine Average Gravity
      (Variables|Default|SetAverageGravity "0, 0, 0")
      (if (== (Utilities|Array|Length _overlappingactors) 0)
        (Variables|Default|SetGravityDirection "0, 0,-1.000000")
        (else
          (for _array_element _overlappingactors
            (Variables|Default|SetAverageGravity (+ (* (Transformation|GetActorUpVector _array_element) -1.0) (Variables|Default|GetAverageGravity))))
          (Variables|Default|SetGravityDirection (Math|Vector|Normalize (Variables|Default|GetAverageGravity))))))
    (:then_1
      ;[1 1 1] Add Gravity
      (Physics|AddForce (Variables|Default|GetItemMesh) (* (Variables|Default|GetGravityDirection) (Math|Conversions|ToVector(Float) (Variables|Default|GetGravityStrength))) "None" true))))