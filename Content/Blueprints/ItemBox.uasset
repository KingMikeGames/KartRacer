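; ItemBox is a kart-racing pickup that grants an item to a kart driving into its mesh.
; On overlap, the server asks the RaceMode game mode to generate an item for the kart's KartController.
; After a short delay it stores that item as the controller's current item and flags it as held, only if none is held, then prints the item's class name.
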(event OnComponentBeginOverlap(StaticMesh)
  (params (OtherActor :type Actor%20Object%20Reference) (OtherComp :type Primitive%20Component%20Object%20Reference) (OtherBodyIndex :type Integer) (bFromSweep :type Boolean) (SweepResult :type Hit%20Result%20Structure%20%28by%20ref%29))
  (Networking|SwitchHasAuthority
    (:Authority
      (bind _asbase_kart (Utilities|Casting|CastToBaseKart OtherActor))
      (bind _asrace_mode (Utilities|Casting|CastToRaceMode (Game|GetGameMode)))
      (bind _askart_controller (Utilities|Casting|CastToKartController (Pawn|GetController _asbase_kart)))
      (bind _item (Default|GenerateItem _asrace_mode))
      (Utilities|FlowControl|Delay 0.2)
      (if (not (Variables|/Game/PlayerController/KartController.KartController_C|GetHasItem _askart_controller))
        (bind _output_get (Variables|/Game/PlayerController/KartController.KartController_C|SetCurrentItem _askart_controller _item))
        (Variables|/Game/PlayerController/KartController.KartController_C|SetHasItem _askart_controller true)
        (Development|PrintString (Utilities|GetClassDisplayName (.item _output_get)))))))

(event EventBeginPlay)

(event EventActorBeginOverlap
  (params (OtherActor :type Actor%20Object%20Reference)))

(event EventTick
  (params (DeltaSeconds :type Float%20%28single-precision%29)))

(fn ConstructionScript)