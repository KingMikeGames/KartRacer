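; FinishLine is a lap trigger actor for a kart race that decides when a kart completes a lap.
; On BeginPlay it counts every CheckPoint actor in the level.
; When a Kart overlaps it, it calls LapGet on the KartController if that controller's checkpoint count matches the total and its race is unfinished.
; The controller's checkpoint list is cleared on every crossing, whether or not the lap counts.
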(event Collision|EventActorBeginOverlap
  (params (OtherActor :type Actor%20Object%20Reference))
  (bind _askart (Utilities|Casting|CastToKart OtherActor))
  (bind _askart_controller (Utilities|Casting|CastToKartController (Pawn|GetController _askart)))
  (if (and (== (Utilities|Array|Length (Variables|/Game/PlayerController/KartController.KartController_C|GetCheckpoints _askart_controller)) (Variables|Default|GetNumberOfCheckpoints)) (not (Variables|/Game/PlayerController/KartController.KartController_C|GetRaceFinished _askart_controller)))
    (Default|LapGet _askart_controller)
    (Utilities|Array|Clear (Variables|/Game/PlayerController/KartController.KartController_C|GetCheckpoints _askart_controller))
    (else
      (Utilities|Array|Clear (Variables|/Game/PlayerController/KartController.KartController_C|GetCheckpoints _askart_controller)))))

(event EventBeginPlay
  (bind _outactors (Actor|GetAllActorsOfClass "/Game/Blueprints/CheckPoint.CheckPoint_C"))
  (Variables|Default|SetNumberOfCheckpoints (Utilities|Array|Length _outactors)))

(fn ConstructionScript)