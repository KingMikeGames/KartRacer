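; Item pickup actor that shatters and disappears when a BP_BaseKart drives into it; no item is granted in this graph.
; Sphere overlap applies very large damage with zero impulse to ItemDM, apparently a destructible mesh, to break it in place.
; It also stops the rotating movement, hides the billboard and deactivates the point light.
; The actor destroys itself after a short delay.
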(event OnComponentBeginOverlap(Sphere)
  (params (OtherActor :type Actor%20Object%20Reference) (OtherComp :type Primitive%20Component%20Object%20Reference) (OtherBodyIndex :type Integer) (bFromSweep :type Boolean) (SweepResult :type Hit%20Result%20Structure%20%28by%20ref%29))
  ;[1 1 1] Item Get
  (Utilities|Casting|CastToBP_BaseKart OtherActor)
  (Game|Damage|ApplyDamage (Variables|Default|GetItem_DM) 2e+05 (Math|Vector|MakeVector 0.0 0.0 0.0) (Math|Vector|MakeVector 0.0 0.0 0.0) 0.0)
  (Variables|/Script/Engine.RotatingMovementComponent|SetRotationRate (Variables|Default|GetRotatingMovement) "0, 0, 0")
  (Development|SetHiddeninGame (Variables|Default|GetBillboard) true false)
  (Components|Activation|SetActive (Variables|Default|GetPointLight) false false)
  (Utilities|FlowControl|Delay 2.0)
  (Actor|DestroyActor))

(event EventBeginPlay)

(event EventActorBeginOverlap
  (params (OtherActor :type Actor%20Object%20Reference)))

(event EventTick
  (params (DeltaSeconds :type Float%20%28single-precision%29)))

(fn ConstructionScript)