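; BP_Kart is a drivable physics kart that accelerates and steers by applying force and torque to its static mesh from axis input.
; Each tick, four corner arrows line-trace as suspension, averaging ground height and normals.
; While any wheel is grounded, it sets the mesh height directly, interpolates rotation to the slope and cancels velocity along its up axis.
; A counter-force on sideways velocity provides lateral grip, even airborne.
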(event EventBeginPlay
  (Utilities|Array|AddUnique (Variables|Default|GetWheelArray) (Variables|Default|GetFrontLeftArrow))
  (Utilities|Array|AddUnique (Variables|Default|GetWheelArray) (Variables|Default|GetBackLeftArrow))
  (Utilities|Array|AddUnique (Variables|Default|GetWheelArray) (Variables|Default|GetBackRightArrow))
  (Utilities|Array|AddUnique (Variables|Default|GetWheelArray) (Variables|Default|GetFrontRightArrow))
  (Variables|Default|SetLastRotation (Transformation|GetWorldRotation (Variables|Default|GetStaticMesh))))

(event EventActorBeginOverlap
  (params (OtherActor :type Actor%20Object%20Reference)))

(event EventTick
  (params (DeltaSeconds :type Float%20%28single-precision%29))
  (bind _staticmesh (Variables|Default|GetStaticMesh))
  (bind _staticmesh_2 (Variables|Default|GetStaticMesh))
  (bind _staticmesh_3 (Variables|Default|GetStaticMesh))
  (bind _staticmesh_4 (Variables|Default|GetStaticMesh))
  (bind _staticmesh_5 (Variables|Default|GetStaticMesh))
  (bind _returnvalue (Math|Vector|GetRightVector _staticmesh_5))
  (bind _returnvalue_2 (Transformation|GetWorldLocation _staticmesh_2))
  (bind _returnvalue_3 (Math|Vector|GetUpVector _staticmesh_4))
  (bind _returnvalue_4 (* _returnvalue_3 -1.0))
  (Utilities|FlowControl|Sequence
    (:then_0
      (Variables|Default|SetAverageHeight 0.0)
      (Variables|Default|SetAverageUp "0, 0, 0")
      (Variables|Default|SetGroundedWheels 0)
      (for _array_element (Variables|Default|GetWheelArray)
        (Transformation|SetRelativeLocation _array_element "0, 0, 0" false false)
        (bind (_outhit _returnvalue_5) (Collision|LineTraceByChannel (Transformation|GetWorldLocation _array_element) (+ (Transformation|GetWorldLocation _array_element) (* (Math|Vector|GetForwardVector _array_element) (Variables|Default|GetSuspensionHeight))) "TraceTypeQuery1" false 0 "None"))
        (if _returnvalue_5
          (Variables|Default|SetAverageUp (+ (.normal _outhit) (Variables|Default|GetAverageUp)))
          (Variables|Default|SetAverageHeight (+ (.Z (Math|Vector|BreakVector (.location _outhit))) (Variables|Default|GetAverageHeight)))
          (if _returnvalue_5
            (Math|Integer|IncrementInt (Variables|Default|GetGroundedWheels)))
          (else
            (Variables|Default|SetAverageHeight (+ (+ (.Z (Math|Vector|BreakVector (+ (Transformation|GetWorldLocation _array_element) (* (Math|Vector|GetForwardVector _array_element) (Variables|Default|GetSuspensionHeight))))) 15.0) (Variables|Default|GetAverageHeight))))))
      (if (> (Variables|Default|GetGroundedWheels) 0)
        (Transformation|SetWorldLocationAndRotation _staticmesh_2 (Math|Vector|MakeVector (.x _returnvalue_2) (.y _returnvalue_2) (+ (/ (Variables|Default|GetAverageHeight) 4.0) 75.0)) (Class|KismetMathLibrary|RInterptoConstant (Variables|Default|GetLastRotation) (Math|Rotator|MakeRotator (.roll (Math|Rotator|MakeRotfromXZ (Math|Vector|GetForwardVector _staticmesh_3) (Math|Vector|Normalize (Variables|Default|GetAverageUp)))) (.pitch (Class|KismetMathLibrary|MakeRotfromYZ (Math|Vector|GetRightVector _staticmesh_3) (Math|Vector|Normalize (Variables|Default|GetAverageUp)))) (.yaw (Math|Rotator|MakeRotator 0.0 0.0 (.yaw (Transformation|GetWorldRotation _staticmesh_3))))) DeltaSeconds 1.5e+02) false false)
        (Variables|Default|SetLastRotation (Transformation|GetWorldRotation _staticmesh_4))
        (bind _returnvalue_6 (Physics|GetPhysicsLinearVelocity (Variables|Default|GetStaticMesh) "None"))
        (bind _returnvalue_7 (Physics|GetPhysicsLinearVelocity _staticmesh "None"))
        (Physics|SetPhysicsLinearVelocity _staticmesh (- _returnvalue_7 (* _returnvalue_4 (Math|Conversions|ToVector(Float) (Math|Vector|DotProduct _returnvalue_6 _returnvalue_4)))) false "None")))
    (:then_1
      (bind _returnvalue_8 (Physics|GetPhysicsLinearVelocity _staticmesh_5 "None"))
      (Physics|AddForce _staticmesh_5 (* (* _returnvalue (* (Math|Vector|DotProduct _returnvalue_8 _returnvalue) -1.0)) 2.0) "None" true))))

(event Input|AxisEvents|InputAxisTurn
  (params (AxisValue :type Float%20%28single-precision%29))
  (bind _staticmesh (Variables|Default|GetStaticMesh))
  (Class|PrimitiveComponent|AddTorque _staticmesh (* (* (Math|Vector|GetUpVector _staticmesh) (Variables|Default|GettorqueForce)) AxisValue) "None" true))

(event Input|AxisEvents|InputAxisAccelerate
  (params (AxisValue :type Float%20%28single-precision%29))
  (bind _staticmesh (Variables|Default|GetStaticMesh))
  (Physics|AddForce _staticmesh (* (* (Math|Vector|GetForwardVector _staticmesh) (Variables|Default|GetAccelForce)) AxisValue) "None" true))

(fn ConstructionScript)