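; Kart Blueprint that simulates four-wheel suspension visuals, fitting wheels to the ground and tilting the body to match.
; The construction script builds wheel and arrow arrays; each Tick sphere-traces along the arrows to place wheels and record compression and grounding.
; Wheel-position vectors then set body pitch and roll directly, preserving yaw.
; Height and normal averages are accumulated but unused; interpolated rotation and body-location nodes are disconnected, with no driving logic.
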(event EventBeginPlay)

(event EventTick
  (params (DeltaSeconds :type Float%20%28single-precision%29))
  (bind _bodymesh (Variables|Default|GetBodyMesh))
  (bind _wheelarray (Variables|Arrays|GetWheelArray))
  (bind _wheelarray_2 (Variables|Arrays|GetWheelArray))
  (bind _suspensionheight (Variables|Physics|GetSuspensionHeight))
  (Utilities|FlowControl|Sequence
    (:then_0
      ;[1 1 1] Reset Transform Values
      (Variables|Transform|SetAverageHeight 0.0)
      (Variables|Transform|SetAverageUp "0, 0, 0")
      (Variables|Physics|SetGroundedWheels 0))
    (:then_1
      ;[1 1 1] Get height, normals and set wheel locations
      (for (_array_element _array_index) (Variables|Arrays|GetTraceArrowArray)
        (Variables|PretendLocals|SetCurrentWheelIndex _array_index)
        (bind (_outhit _returnvalue) (Class|KismetSystemLibrary|SphereTraceSingleNEW (Transformation|GetWorldLocation _array_element) (+ (Transformation|GetWorldLocation _array_element) (* (Math|Vector|GetForwardVector _array_element) (Variables|Physics|GetSuspensionHeight))) (Variables|Physics|GetWheelRadius) "TraceTypeQuery1" false 0 "None" true))
        (if _returnvalue
          (Variables|Transform|SetAverageUp (+ (.impactnormal _outhit) (Variables|Transform|GetAverageUp)))
          (Variables|Transform|SetAverageHeight (+ (- _suspensionheight (* (.time _outhit) _suspensionheight)) (Variables|Transform|GetAverageHeight)))
          (Transformation|SetWorldLocation (.wheelmesh (Utilities|Array|Get(acopy) (Variables|Arrays|GetWheelArray) (Variables|PretendLocals|GetCurrentWheelIndex))) (.location _outhit) false false)
          (Utilities|Array|SetArrayElem (Variables|Arrays|GetWheelArray) (Variables|PretendLocals|GetCurrentWheelIndex) (Utilities|Struct|MakeWheelStruct (.wheelmesh (Utilities|Array|Get(acopy) (Variables|Arrays|GetWheelArray) (Variables|PretendLocals|GetCurrentWheelIndex))) (.time _outhit) (select (== (.time _outhit) 1.0) false true)))
          (if (select (== (.time _outhit) 1.0) false true)
            (Math|Integer|IncrementInt (Variables|Physics|GetGroundedWheels)))
          (else
            (Variables|Transform|SetAverageUp (Math|Vector|GetForwardVector (Utilities|Array|Get(acopy) (Variables|Arrays|GetArrowTiltArray) (Variables|PretendLocals|GetCurrentWheelIndex))))
            (Transformation|SetWorldLocation (.wheelmesh (Utilities|Array|Get(acopy) (Variables|Arrays|GetWheelArray) (Variables|PretendLocals|GetCurrentWheelIndex))) (+ (Transformation|GetWorldLocation _array_element) (* (Math|Vector|GetForwardVector _array_element) (Variables|Physics|GetSuspensionHeight))) false false)))))
    (:then_2
      (Variables|Default|SetForwardVector (Math|Vector|Normalize (- (Transformation|GetWorldLocation (.wheelmesh (Utilities|Array|Get(acopy) _wheelarray_2))) (Transformation|GetWorldLocation (.wheelmesh (Utilities|Array|Get(acopy) _wheelarray_2 2))))))
      (Variables|Default|SetRightVector (Math|Vector|Normalize (- (Transformation|GetWorldLocation (.wheelmesh (Utilities|Array|Get(acopy) _wheelarray 1))) (Transformation|GetWorldLocation (.wheelmesh (Utilities|Array|Get(acopy) _wheelarray))))))
      (Variables|Transform|SetLastRotation (Transformation|GetWorldRotation _bodymesh))
      (Transformation|SetWorldRotation _bodymesh (Math|Rotator|MakeRotator (.roll (Math|Rotator|MakeRotfromXZ (Variables|Default|GetForwardVector) (Math|Vector|Normalize (Math|Vector|CrossProduct (Variables|Default|GetForwardVector) (Variables|Default|GetRightVector))))) (.pitch (Class|KismetMathLibrary|MakeRotfromYZ (Variables|Default|GetRightVector) (Math|Vector|Normalize (Math|Vector|CrossProduct (Variables|Default|GetForwardVector) (Variables|Default|GetRightVector))))) (.yaw (Math|Rotator|MakeRotator 0.0 0.0 (.yaw (Transformation|GetWorldRotation (Variables|Default|GetBodyMesh)))))) false false))))

(fn ConstructionScript
  (bind _wheelarray (Variables|Arrays|GetWheelArray))
  (bind _arrowtiltarray (Variables|Arrays|GetArrowTiltArray))
  (bind _tracearrowarray (Variables|Arrays|GetTraceArrowArray))
  (Utilities|FlowControl|Sequence
    (:then_0
      ;[1 1 1] Initialize WheelMeshArray
      (Utilities|Array|AddUnique _wheelarray (Utilities|Struct|MakeWheelStruct (Variables|Default|GetFrontLeftWheelMesh) 0.0 false))
      (Utilities|Array|AddUnique _wheelarray (Utilities|Struct|MakeWheelStruct (Variables|Default|GetFrontRightWheelMesh) 0.0 false))
      (Utilities|Array|AddUnique _wheelarray (Utilities|Struct|MakeWheelStruct (Variables|Default|GetBackLeftWheelMesh) 0.0 false))
      (Utilities|Array|AddUnique _wheelarray (Utilities|Struct|MakeWheelStruct (Variables|Default|GetBackRightWheelMesh) 0.0 false)))
    (:then_1
      ;[1 1 1] Initialize Arrow Tilt array
      (Utilities|Array|AddUnique _arrowtiltarray (Variables|Default|GetFrontLeftTilt))
      (Utilities|Array|AddUnique _arrowtiltarray (Variables|Default|GetFrontRightTilt))
      (Utilities|Array|AddUnique _arrowtiltarray (Variables|Default|GetBackLeftTilt))
      (Utilities|Array|AddUnique _arrowtiltarray (Variables|Default|GetBackRightTilt)))
    (:then_2
      ;[1 1 1] Initialize Arrow array for tracing wheels
      (Utilities|Array|AddUnique _tracearrowarray (Variables|Default|GetFrontLeftWheel))
      (Utilities|Array|AddUnique _tracearrowarray (Variables|Default|GetFrontRightWheel))
      (Utilities|Array|AddUnique _tracearrowarray (Variables|Default|GetBackLeftWheel))
      (Utilities|Array|AddUnique _tracearrowarray (Variables|Default|GetBackRightWheel)))))