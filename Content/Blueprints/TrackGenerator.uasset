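; Spline-driven track generator that builds a road with optional left and right guard rails in the construction script.
; It resizes RoadDataArray to match the spline point count, giving each point bank, width, thickness and rail settings.
; BuildTrackElement adds a spline mesh per segment, blending roll and scale between neighbouring points, with optional loop closure and collision.
; An optional overlay labels each point with its index.
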(event EventBeginPlay)

(event EventActorBeginOverlap
  (params (OtherActor :type Actor%20Object%20Reference)))

(event EventTick
  (params (DeltaSeconds :type Float%20%28single-precision%29)))

(fn ConstructionScript
  (bind _roaddataarray (Variables|Default|GetRoadDataArray))
  (Utilities|FlowControl|Sequence
    (:then_0
      ;[1 1 1] Store number of splinepoints
      (Variables|Default|SetNumberOfSplinePoints (Spline|GetNumberOfSplinePoints (Variables|Default|GetSpline))))
    (:then_1
      ;[1 1 1] Build road data array
      (Math|Integer|CompareInt (Utilities|Array|Length (Variables|Default|GetRoadDataArray)) (Variables|Default|GetNumberOfSplinePoints) :!label _label
        (:>
          (Utilities|Array|RemoveIndex _roaddataarray (Utilities|Array|LastIndex _roaddataarray))
          (goto _label))
        (:<
          (Utilities|Array|Add (Variables|Default|GetRoadDataArray) (Variables|Default|GetRoadMeshDefaults))
          (goto _label))))
    (:then_2
      ;[1 1 1] Loop the for
      (for _index (range 0 (- (Variables|Default|GetNumberOfSplinePoints) (select (Variables|Default|GetLoop) 1 2)))
        ;[1 1 1] Store Draw Left Right Guard Rails
        (Variables|Default|SetCurrentLoopIndex _index)
        (Variables|Default|SetDrawLeftGuardRail (.leftguardrail (Utilities|Array|Get(acopy) (Variables|Default|GetRoadDataArray) (Variables|Default|GetCurrentLoopIndex))))
        (Variables|Default|SetDrawRightGuardRail (.righguardrail (Utilities|Array|Get(acopy) (Variables|Default|GetRoadDataArray) (Variables|Default|GetCurrentLoopIndex))))
        (Utilities|FlowControl|Sequence
          (:then_0
            ;[1 1 1] DrawRoadMesh
            (CallFunction|BuildTrackElement (Variables|Default|GetCurrentLoopIndex) (Variables|Default|GetRoadMesh)))
          (:then_1
            ;[1 1 1] Draw left guard rail
            (if (Variables|Default|GetDrawLeftGuardRail)
              (CallFunction|BuildTrackElement (Variables|Default|GetCurrentLoopIndex) (Variables|Default|GetLeftGuardRailMesh))))
          (:then_2
            ;[1 1 1] Draw Right Guard Rail
            (if (Variables|Default|GetDrawRightGuardRail)
              (CallFunction|BuildTrackElement (Variables|Default|GetCurrentLoopIndex) (Variables|Default|GetRightGuardRailMesh)))))))
    (:then_3
      ;[1 1 1] Draw Text above spline points
      (if (Variables|Default|GetDrawTrackPointNumbers)
        (for _index_2 (range 0 (- (Variables|Default|GetNumberOfSplinePoints) 1))
          (Variables|Default|SetCurrentTrackPoint (Utilities|Text|ToText(Integer) _index_2))
          (bind _returnvalue (AddComponent|AddTextRenderComponent false (Math|Transform|MakeTransform (Math|Vector|MakeVector (.X (Math|Vector|BreakVector (.Location (Spline|GetLocationandTangentatSplinePoint (Variables|Default|GetSpline) _index_2 "Local")))) (.Y (Math|Vector|BreakVector (.Location (Spline|GetLocationandTangentatSplinePoint (Variables|Default|GetSpline) _index_2 "Local")))) (+ (.Z (Math|Vector|BreakVector (.Location (Spline|GetLocationandTangentatSplinePoint (Variables|Default|GetSpline) _index_2 "Local")))) 5e+01)) (Math|Conversions|RotationFromXVector (* (.Tangent (Spline|GetLocationandTangentatSplinePoint (Variables|Default|GetSpline) _index_2 "Local")) -1.0)))))
          (Rendering|Components|TextRender|SetText _returnvalue (Variables|Default|GetCurrentTrackPoint)))))))

(fn BuildTrackElement
  (params (NewParam :type Integer) (TrackElementMesh :type Static%20Mesh%20Object%20Reference))
  ;[1 1 1] store Inputs in local variables
  (LocalVariables|SetLocal_TrackElementMesh TrackElementMesh)
  (LocalVariables|SetLocal_CurrentLoopIndex NewParam)
  (LocalVariables|SetLocal_NextLoopIndex (Math|Integer|%(Integer) (+ NewParam 1) (Variables|Default|GetNumberOfSplinePoints)))
  (Utilities|FlowControl|Sequence
    (:then_0
      ;[1 1 1] Store data to build track
      (LocalVariables|SetLocal_StartLocation (.Location (Spline|GetLocationandTangentatSplinePoint (Variables|Default|GetSpline) (LocalVariables|GetLocal_CurrentLoopIndex) "Local")))
      (LocalVariables|SetLocal_StartTangent (.Tangent (Spline|GetLocationandTangentatSplinePoint (Variables|Default|GetSpline) (LocalVariables|GetLocal_CurrentLoopIndex) "Local")))
      (LocalVariables|SetLocal_EndLocation (.Location (Spline|GetLocationandTangentatSplinePoint (Variables|Default|GetSpline) (LocalVariables|GetLocal_NextLoopIndex) "Local")))
      (LocalVariables|SetLocal_EndTangent (.Tangent (Spline|GetLocationandTangentatSplinePoint (Variables|Default|GetSpline) (LocalVariables|GetLocal_NextLoopIndex) "Local")))
      (LocalVariables|SetLocal_StartRoll (.bank (Utilities|Array|Get(acopy) (Variables|Default|GetRoadDataArray) (LocalVariables|GetLocal_CurrentLoopIndex))))
      (LocalVariables|SetLocal_StartScale (Math|Vector2D|MakeVector2D (.trackwidth (Utilities|Array|Get(acopy) (Variables|Default|GetRoadDataArray) (LocalVariables|GetLocal_CurrentLoopIndex))) (.trackthickness (Utilities|Array|Get(acopy) (Variables|Default|GetRoadDataArray) (LocalVariables|GetLocal_CurrentLoopIndex)))))
      (LocalVariables|SetLocal_EndRoll (.bank (Utilities|Array|Get(acopy) (Variables|Default|GetRoadDataArray) (LocalVariables|GetLocal_NextLoopIndex))))
      (LocalVariables|SetLocal_EndScale (Math|Vector2D|MakeVector2D (.trackwidth (Utilities|Array|Get(acopy) (Variables|Default|GetRoadDataArray) (LocalVariables|GetLocal_NextLoopIndex))) (.trackthickness (Utilities|Array|Get(acopy) (Variables|Default|GetRoadDataArray) (LocalVariables|GetLocal_NextLoopIndex))))))
    (:then_1
      ;[1 1 1] Generate the actual meshes
      (bind _returnvalue (AddComponent|AddSplineMeshComponent false))
      (bind _output_get (LocalVariables|SetLocal_CurrentSplineMesh _returnvalue))
      (Components|StaticMesh|SetStaticMesh _output_get (LocalVariables|GetLocal_TrackElementMesh))
      (SplineMesh|SetStartandEnd (LocalVariables|GetLocal_CurrentSplineMesh) (LocalVariables|GetLocal_StartLocation) (LocalVariables|GetLocal_StartTangent) (LocalVariables|GetLocal_EndLocation) (LocalVariables|GetLocal_EndTangent) true :!class /Script/Engine.SplineMeshComponent)
      (Class|SplineMeshComponent|SetStartRoll (LocalVariables|GetLocal_CurrentSplineMesh) (LocalVariables|GetLocal_StartRoll) true)
      (Class|SplineMeshComponent|SetEndRoll (LocalVariables|GetLocal_CurrentSplineMesh) (LocalVariables|GetLocal_EndRoll) true)
      (SplineMesh|SetStartScale (LocalVariables|GetLocal_CurrentSplineMesh) (LocalVariables|GetLocal_StartScale) true :!class /Script/Engine.SplineMeshComponent)
      (SplineMesh|SetEndScale (LocalVariables|GetLocal_CurrentSplineMesh) (LocalVariables|GetLocal_EndScale) true :!class /Script/Engine.SplineMeshComponent)
      (Collision|SetCollisionEnabled (LocalVariables|GetLocal_CurrentSplineMesh) (select (Variables|Default|GetCollisions) "QueryAndPhysics" "NoCollision")))))