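; Podium Blueprint that holds twelve ordered placement spots, First through Twelfth, apparently for standings.
; On BeginPlay it inserts each spot into the Locations array at its zero-based rank, so First lands at index 0.
; It only builds this lookup list; nothing in these graphs reads it or places anything, and the construction script is empty.
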(event EventBeginPlay
  (Utilities|Array|Insert (Variables|Default|GetLocations) (Variables|Default|GetFirst))
  (Utilities|Array|Insert (Variables|Default|GetLocations) (Variables|Default|GetSecond) 1)
  (Utilities|Array|Insert (Variables|Default|GetLocations) (Variables|Default|GetThird) 2)
  (Utilities|Array|Insert (Variables|Default|GetLocations) (Variables|Default|GetFourth) 3)
  (Utilities|Array|Insert (Variables|Default|GetLocations) (Variables|Default|GetFifth) 4)
  (Utilities|Array|Insert (Variables|Default|GetLocations) (Variables|Default|GetSixth) 5)
  (Utilities|Array|Insert (Variables|Default|GetLocations) (Variables|Default|GetSeventh) 6)
  (Utilities|Array|Insert (Variables|Default|GetLocations) (Variables|Default|GetEigth) 7)
  (Utilities|Array|Insert (Variables|Default|GetLocations) (Variables|Default|GetNinth) 8)
  (Utilities|Array|Insert (Variables|Default|GetLocations) (Variables|Default|GetTenth) 9)
  (Utilities|Array|Insert (Variables|Default|GetLocations) (Variables|Default|GetEleventh) 10)
  (Utilities|Array|Insert (Variables|Default|GetLocations) (Variables|Default|GetTwelvth) 11))

(fn ConstructionScript)